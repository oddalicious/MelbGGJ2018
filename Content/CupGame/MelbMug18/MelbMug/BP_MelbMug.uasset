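; BP_MelbMug is a player-controlled mug character that walks and turns via input axes and makes surface-dependent impact sounds.
; Movement input pushes it along its yaw-only forward vector, while Rotation input accumulates a look yaw applied every Tick.
; Tick also toggles CanRun on ABP_MelbMug from the movement axis.
; Capsule hits play a sound chosen by physical surface type, though hits without a physical material play nothing.
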(event OnComponentHit(CapsuleComponent)
  (params (HitComponent :type Primitive%20Component%20Object%20Reference) (OtherActor :type Actor%20Object%20Reference) (OtherComp :type Primitive%20Component%20Object%20Reference) (NormalImpulse :type Vector :default "0, 0, 0") (Hit :type Hit%20Result%20Structure%20%28by%20ref%29))
  (bind (_bblockinghit _binitialoverlap _time _distance _location _impactpoint _normal _impactnormal _physmat) (Collision|BreakHitResult Hit))
  (Utilities|IsValid _physmat
    (:Is%20Valid
      (bind _outclip (CallFunction|GetAudioforPhysicsMaterial (Variables|/Script/Engine.PhysicalMaterial|GetSurfaceType _physmat)))
      (Audio|PlaySoundatLocation _outclip _location))
    (:Is%20Not%20Valid
      (CallFunction|GetAudioforPhysicsMaterial "SurfaceType_Default"))))

(event EventTick
  (params (DeltaSeconds :type Float%20%28single-precision%29))
  (bind _mesh (Variables|Character|GetMesh))
  (bind _returnvalue (Components|SkeletalMesh|GetAnimInstance _mesh))
  (Utilities|FlowControl|Sequence
    (:then_0
      (Transformation|SetActorRotation (Variables|Default|GetLookRotation)))
    (:then_1
      (if (!= (Input|AxisValues|GetMovement) 0.0)
        (bind _asabp_melb_mug (Utilities|Casting|CastToABP_MelbMug _returnvalue))
        (Variables|/Game/CupGame/MelbMug18/MelbMug/ABP_MelbMug.ABP_MelbMug_C|SetcanRun _asabp_melb_mug true)
        (else
          (bind _asabp_melb_mug_2 (Utilities|Casting|CastToABP_MelbMug _returnvalue))
          (Variables|/Game/CupGame/MelbMug18/MelbMug/ABP_MelbMug.ABP_MelbMug_C|SetcanRun _asabp_melb_mug_2 false))))))

(event Input|AxisEvents|InputAxisMovement
  (params (AxisValue :type Float%20%28single-precision%29))
  (bind _output_get (Variables|Default|SetCurrentVelocity AxisValue))
  (Pawn|Input|AddMovementInput (Math|Vector|GetForwardVector (Math|Rotator|MakeRotator 0.0 0.0 (.yaw (Transformation|GetActorRotation)))) (* _output_get (Variables|Default|GetSpeed)) false))

(event Input|AxisEvents|InputAxisRotation
  (params (AxisValue :type Float%20%28single-precision%29))
  (Variables|Default|SetLookRotation (Math|Rotator|MakeRotator (.roll (Variables|Default|GetLookRotation)) (.pitch (Variables|Default|GetLookRotation)) (+ (.yaw (Variables|Default|GetLookRotation)) (* (Variables|Default|GetrotateSpeed) AxisValue)))))

(fn ConstructionScript)

(fn GetAudioforPhysicsMaterial
  (params (Material :type EPhysicalSurface%20Enum :default "SurfaceType_Default"))
  (switch Utilities|FlowControl|Switch|SwitchonEPhysicalSurface Material
    (:SurfaceType_Default
      (LocalVariables|Setclip (Variables|Default|GetCeramicSound) :!label _label)
      (return (LocalVariables|Getclip)))
    (:SurfaceType1
      (goto _label))
    (:SurfaceType2
      (LocalVariables|Setclip (Variables|Default|GetPlasticSound))
      (return (LocalVariables|Getclip)))
    (:SurfaceType3
      (LocalVariables|Setclip (Variables|Default|GetWoodSound))
      (return (LocalVariables|Getclip)))
    (:SurfaceType4
      (LocalVariables|Setclip (Variables|Default|GetMetalSound))
      (return (LocalVariables|Getclip)))
    (:SurfaceType5
      (LocalVariables|Setclip (Variables|Default|GetGlassSound)))))