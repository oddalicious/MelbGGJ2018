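; MusicManager in CupGame switches the soundtrack between regular and spotted music depending on whether the player has been spotted.
; HasBeenSpotted plays a 2D sting, throttled by a short cooldown that Tick counts down, then restarts the spotted track and increments a spot counter.
; LoseSpot decrements the counter and restores regular music at zero, and also runs at BeginPlay to start it.
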(event EventBeginPlay
  (CallFunction|LoseSpot))

(event EventTick
  (params (DeltaSeconds :type Float%20%28single-precision%29))
  (CallFunction|TickDownScare DeltaSeconds))

(fn ConstructionScript)

(fn PlaySpotSound
  (Audio|PlaySound2D self (Variables|Default|GetSpotSound)))

(fn LoseSpot
  (bind _regularmusic (Variables|Default|GetRegularMusic))
  (bind _audio (Variables|Default|GetAudio))
  (bind _output_get (Variables|Default|SetspotCount (Math|Integer|Max(Integer) (- (Variables|Default|GetspotCount) 1))))
  (if (<= _output_get 0)
    (if (!= (Variables|/Script/Engine.AudioComponent|GetSound _audio) _regularmusic)
      (Audio|Components|Audio|Stop _audio)
      (Variables|/Script/Engine.AudioComponent|SetSound _audio _regularmusic)
      (Audio|Components|Audio|Play _audio 0.0))))

(fn SpotPlayer
  (bind _audio (Variables|Default|GetAudio))
  (Audio|Components|Audio|Stop _audio)
  (Variables|/Script/Engine.AudioComponent|SetSound _audio (Variables|Default|GetSpottedMusic))
  (Audio|Components|Audio|Play _audio 0.0)
  (Math|Integer|IncrementInt (Variables|Default|GetspotCount)))

(fn HasBeenSpotted
  (if (== (Variables|Default|GettimeSinceLastScare) 0.0)
    (Audio|PlaySound2D self (Variables|Default|GetSpotSound))
    (Variables|Default|SettimeSinceLastScare 1.5))
  (CallFunction|SpotPlayer))

(fn SetVolume
  (params (volume :type Float%20%28single-precision%29))
  (Audio|Components|Audio|SetVolumeMultiplier (Variables|Default|GetAudio) volume :!class /Script/Engine.AudioComponent))

(fn TickDownScare
  (params (B :type Float%20%28single-precision%29))
  (Variables|Default|SettimeSinceLastScare (Math|Float|Max(Float) (- (Variables|Default|GettimeSinceLastScare) B) 0.0)))