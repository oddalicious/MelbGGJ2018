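; Player-controlled mug character with forward-only movement, yaw turning and clamped camera pitch, reporting itself noticeable while moving, rotating or animating.
; Tick applies rotations, updates ABP_MelbMug's run flag and positions a world-level plane as liquid at the fill amount.
; Helpers add fill, spawn coffee drops when nearly full and play mug sounds, while capsule hits choose audio by surface type.
; It also creates instruction, pause, win and loss widgets that pause play.
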(event OnComponentHit(CapsuleComponent)
  (params (HitComponent :type Primitive%20Component%20Object%20Reference) (OtherActor :type Actor%20Object%20Reference) (OtherComp :type Primitive%20Component%20Object%20Reference) (NormalImpulse :type Vector :default "0, 0, 0") (Hit :type Hit%20Result%20Structure%20%28by%20ref%29))
  (bind (_bblockinghit _binitialoverlap _time _distance _location _impactpoint _normal _impactnormal _physmat) (Collision|BreakHitResult Hit))
  (Utilities|IsValid _physmat
    (:Is%20Valid
      (bind _outclip (CallFunction|GetAudioforPhysicsMaterial (Variables|/Script/Engine.PhysicalMaterial|GetSurfaceType _physmat)))
      (Audio|PlaySoundatLocation _outclip _location))
    (:Is%20Not%20Valid
      (CallFunction|GetAudioforPhysicsMaterial "SurfaceType_Default"))))

(event EventBeginPlay
  (Variables|Default|SettargetControlRotation (Variables|Default|GettargetControlRotation))
  (bind _asabp_melb_mug (Utilities|Casting|CastToABP_MelbMug (Components|SkeletalMesh|GetAnimInstance (Variables|Character|GetMesh))))
  (Variables|Default|Setanim _asabp_melb_mug)
  (CallFunction|CreatePauseWidget (Game|GetPlayerController 0))
  (CallFunction|CreateWinWidget)
  (CallFunction|CreateLossWidget)
  (CallFunction|ShowInstructions))

(event EventTick
  (params (DeltaSeconds :type Float%20%28single-precision%29))
  (CallFunction|SetRotations)
  (Variables|/Game/CupGame/Blueprints/ABP_MelbMug.ABP_MelbMug_C|SetcanRun (Variables|Default|Getanim) (Utilities|ShouldAnimate))
  (CallFunction|SetPlaneTransform))

(event Input|ActionEvents|InputActionPaused
  (params (Key :type Key%20Structure))
  (bind _pausewidget (Variables|Default|GetPauseWidget))
  (:Pressed
    (if (not (Game|IsGamePaused))
      (Widget|SetVisibility _pausewidget "Visible")
      (Game|SetGamePaused true)
      (Input|SetInputModeUIOnly (Game|GetPlayerController 0) _pausewidget "LockOnCapture"))))

(event Input|AxisEvents|InputAxisMovement
  (params (AxisValue :type Float%20%28single-precision%29))
  (if (Variables|Default|GetcanMove)
    (CallFunction|MovePlayer AxisValue)))

(event Input|AxisEvents|InputAxisVerticalRotation
  (params (AxisValue :type Float%20%28single-precision%29))
  (CallFunction|SetVerticalRotation AxisValue))

(event Input|AxisEvents|InputAxisHorizontalRotation
  (params (AxisValue :type Float%20%28single-precision%29))
  (if (Variables|Default|GetcanMove)
    (CallFunction|SetHorizontalRotation AxisValue)))

(fn ConstructionScript)

(fn GetAudioforPhysicsMaterial
  (params (Material :type EPhysicalSurface%20Enum :default "SurfaceType_Default"))
  (switch Utilities|FlowControl|Switch|SwitchonEPhysicalSurface Material
    (:SurfaceType_Default
      (LocalVariables|Setclip (Variables|Default|GetCeramicSound) :!label _label)
      (return (LocalVariables|Getclip)))
    (:SurfaceType1
      (goto _label))
    (:SurfaceType2
      (LocalVariables|Setclip (Variables|Default|GetPlasticSound))
      (return (LocalVariables|Getclip)))
    (:SurfaceType3
      (LocalVariables|Setclip (Variables|Default|GetWoodSound))
      (return (LocalVariables|Getclip)))
    (:SurfaceType4
      (LocalVariables|Setclip (Variables|Default|GetMetalSound))
      (return (LocalVariables|Getclip)))
    (:SurfaceType5
      (LocalVariables|Setclip (Variables|Default|GetGlassSound)))))

(fn SetHorizontalRotation
  (params (B :type Float%20%28single-precision%29))
  (bind _returnvalue (Math|Float|Clamp(Float) B -1.0))
  (Variables|Default|SetisRotating (!= _returnvalue 0.0))
  (Variables|Default|SetLookRotation (Math|Rotator|MakeRotator (.roll (Variables|Default|GetLookRotation)) (.pitch (Variables|Default|GetLookRotation)) (+ (.yaw (Variables|Default|GetLookRotation)) (* (Variables|Default|GetrotateSpeed) _returnvalue)))))

(fn SetVerticalRotation
  (params (Axis :type Float%20%28single-precision%29))
  (bind _lookrotation (Variables|Default|GetLookRotation))
  (bind _output_get (Variables|Default|SettargetControlRotation (Math|Rotator|MakeRotator (.roll _lookrotation) (Math|Float|Clamp(Float) (+ (.pitch (Variables|Default|GettargetControlRotation)) (* (select (Variables|Default|GetInvertYAxis) Axis (* Axis -1.0)) (Variables|Default|GetrotateSpeed))) -45.0 1e+01) (.yaw _lookrotation)))))

(fn MovePlayer
  (params (CurrentVelocity :type Float%20%28single-precision%29))
  (bind _returnvalue (> CurrentVelocity 0.0))
  (Variables|Default|SetisMoving _returnvalue)
  (if _returnvalue
    (bind _output_get (Variables|Default|SetCurrentVelocity CurrentVelocity))
    (Pawn|Input|AddMovementInput (Math|Vector|GetForwardVector (Math|Rotator|MakeRotator 0.0 0.0 (.yaw (Transformation|GetActorRotation)))) (* _output_get (Variables|Default|GetSpeed)) false)))

(fn SetRotations
  (bind _returnvalue (Transformation|GetActorRotation))
  (bind _lookrotation (Variables|Default|GetLookRotation))
  (Transformation|SetActorRotation (Math|Rotator|MakeRotator (.roll _lookrotation) (.pitch _lookrotation) (.yaw _lookrotation)))
  (Transformation|SetWorldRotation (Variables|Default|GetSpringArm) (Math|Rotator|MakeRotator (.roll _returnvalue) (.pitch (Variables|Default|GettargetControlRotation)) (.yaw _returnvalue)) false false))

(fn SetPlaneTransform
  (bind _plane (Variables|Default|GetPlane))
  (bind _planemin (Variables|Default|GetplaneMin))
  (bind _fillamount (Variables|Default|GetfillAmount))
  (bind _plane_2 (Variables|Default|GetPlane))
  (bind _relativelocation (Variables|/Script/Engine.SceneComponent|GetRelativeLocation _plane))
  (if (> _fillamount 0.0)
    (Transformation|SetRelativeLocation _plane_2 (Math|Vector|MakeVector (.x _relativelocation) (.y _relativelocation) (+ (* _fillamount (- (Variables|Default|GetplaneMax) _planemin)) _planemin)) false false)
    (Transformation|SetWorldRotation _plane_2 "0, 0, 0" false false)
    (Rendering|SetVisibility _plane_2 true false)
    (else
      (Rendering|SetVisibility _plane false false))))

(fn Fill
  (params (DeltaTime :type Float%20%28single-precision%29) (Length :type Float%20%28single-precision%29))
  (Variables|Default|SetfillAmount (Math|Float|Clamp(Float) (+ (Variables|Default|GetfillAmount) (/ DeltaTime Length)))))

(fn SpawnLeft
  (bind _leftcoffeespawn (Variables|Default|GetLeftCoffeeSpawn))
  (bind _returnvalue (Transformation|GetWorldTransform _leftcoffeespawn))
  (if (>= (Variables|Default|GetfillAmount) 0.9)
    (Game|SpawnActorfromClass "/Game/CoffeeDrop.CoffeeDrop_C" (Math|Transform|MakeTransform (.location _returnvalue) (.rotation _returnvalue)) "Undefined" self 0)))

(fn SpawnRight
  (bind _rightcoffeespawn (Variables|Default|GetRightCoffeeSpawn))
  (bind _returnvalue (Transformation|GetWorldTransform _rightcoffeespawn))
  (if (>= (Variables|Default|GetfillAmount) 0.9)
    (Game|SpawnActorfromClass "/Game/CoffeeDrop.CoffeeDrop_C" (Math|Transform|MakeTransform (.location _returnvalue) (.rotation _returnvalue)) "Undefined" self 0)))

(fn PlayFootstep
  (bind _footstepclips (Variables|Default|GetFootstepClips))
  (Audio|PlaySoundatLocation self (Utilities|Array|Get(acopy) _footstepclips (Math|Random|RandomInteger (Utilities|Array|Length _footstepclips))) (Transformation|GetSocketLocation (Variables|Character|GetMesh) "MugBase")))

(fn GetRandomElement
  (params (NewParam :type Boolean)))

(fn PlayLegPop
  (params (in :type Boolean))
  (Audio|PlaySoundatLocation self (select in (Variables|Default|GetLegPopIn) (Variables|Default|GetLegPopOut)) (Transformation|GetSocketLocation (Variables|Character|GetMesh) "MugBase")))

(fn PlayDrop
  (bind _dropclips (Variables|Default|GetDropClips))
  (Audio|PlaySoundatLocation self (Utilities|Array|Get(acopy) _dropclips (Math|Random|RandomInteger (Utilities|Array|Length _dropclips))) (Transformation|GetSocketLocation (Variables|Character|GetMesh) "MugBase")))

(fn PlaySlosh
  (bind _sloshclips (Variables|Default|GetSloshClips))
  (if (> (Variables|Default|GetfillAmount) 0.0)
    (Audio|PlaySoundatLocation self (Utilities|Array|Get(acopy) _sloshclips (Math|Random|RandomInteger (Utilities|Array|Length _sloshclips))) (Transformation|GetActorLocation))))

(fn CreatePauseWidget
  (params (OwningPlayer :type Player%20Controller%20Object%20Reference))
  (bind _returnvalue (UserInterface|CreateWidget "/Game/GameJamKit/Blueprints/UMG/UMG_GameJam_PauseMenu_Widget.UMG_GameJam_PauseMenu_Widget_C" OwningPlayer))
  (bind _output_get (Variables|Default|SetPauseWidget _returnvalue))
  (UserInterface|Viewport|AddtoViewport _returnvalue 0)
  (Widget|SetVisibility _output_get "Hidden"))

(fn CreateLossWidget
  (bind _returnvalue (UserInterface|CreateWidget "/Game/CupGame/Blueprints/Widgets/LoseGameWidget.LoseGameWidget_C" (Game|GetPlayerController 0)))
  (Variables|Default|SetLoseGameWidget _returnvalue)
  (Widget|SetVisibility _returnvalue "Hidden"))

(fn ShowLoseWidget
  (bind _returnvalue (Game|GetPlayerController 0))
  (bind _losegamewidget (Variables|Default|GetLoseGameWidget))
  (Widget|SetVisibility _losegamewidget "Visible")
  (UserInterface|Viewport|AddtoViewport _losegamewidget 0)
  (Game|SetGamePaused true)
  (Input|SetInputModeUIOnly _returnvalue _losegamewidget "LockOnCapture")
  (Variables|/Script/Engine.PlayerController|SetbShowMouseCursor _returnvalue true))

(fn CreateWinWidget
  (bind _returnvalue (UserInterface|CreateWidget "/Game/CupGame/Blueprints/Widgets/WinGameWidget.WinGameWidget_C" (Game|GetPlayerController 0)))
  (bind _output_get (Variables|Default|SetWinGameWidget _returnvalue))
  (Widget|SetVisibility _output_get "Hidden"))

(fn ShowWinWidget
  (bind _returnvalue (Game|GetPlayerController 0))
  (bind _wingamewidget (Variables|Default|GetWinGameWidget))
  (Widget|SetVisibility _wingamewidget "Visible")
  (UserInterface|Viewport|AddtoViewport _wingamewidget 0)
  (Game|SetGamePaused true)
  (Input|SetInputModeUIOnly _returnvalue _wingamewidget "LockOnCapture")
  (Variables|/Script/Engine.PlayerController|SetbShowMouseCursor _returnvalue true))

(fn IsNoticeAbleFunc
  (return (Math|Boolean|ORBoolean (Variables|Default|GetisMoving) (Variables|Default|GetisRotating) (Variables|/Game/CupGame/Blueprints/ABP_MelbMug.ABP_MelbMug_C|GetisAnimating (Variables|Default|Getanim)))))

(fn ShowInstructions
  (bind _returnvalue (Game|GetPlayerController 0))
  (bind _returnvalue_2 (UserInterface|CreateWidget "/Game/CupGame/Blueprints/Widgets/InstructionsWidget.InstructionsWidget_C" (Game|GetPlayerController 0)))
  (Widget|SetVisibility _returnvalue_2 "Visible")
  (UserInterface|Viewport|AddtoViewport _returnvalue_2 0)
  (Game|SetGamePaused true)
  (Input|SetInputModeUIOnly _returnvalue _returnvalue_2 "LockOnCapture")
  (Variables|/Script/Engine.PlayerController|SetbShowMouseCursor _returnvalue true))