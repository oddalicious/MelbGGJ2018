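; BP_MelbMug is a mug Blueprint in CupGame that supplies an audio clip suited to a physical material.
; GetAudioForPhysicsMaterial switches on the material to pick a ceramic, plastic, wood, metal or glass sound, with ceramic as the default.
; The Rotation input axis event, Tick and construction script are empty, and nothing in this file calls the lookup or plays the clip.
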(event EventTick
  (params (DeltaSeconds :type Float%20%28single-precision%29)))

(event Input|AxisEvents|InputAxisRotation
  (params (AxisValue :type Float%20%28single-precision%29)))

(fn ConstructionScript)

(fn GetAudioforPhysicsMaterial
  (params (Material :type EPhysicalSurface%20Enum :default "SurfaceType_Default"))
  (switch Utilities|FlowControl|Switch|SwitchonEPhysicalSurface Material
    (:SurfaceType_Default
      (LocalVariables|Setclip (Variables|Default|GetCeramicSound) :!label _label)
      (return (LocalVariables|Getclip)))
    (:SurfaceType1
      (goto _label))
    (:SurfaceType2
      (LocalVariables|Setclip (Variables|Default|GetPlasticSound))
      (return (LocalVariables|Getclip)))
    (:SurfaceType3
      (LocalVariables|Setclip (Variables|Default|GetWoodSound))
      (return (LocalVariables|Getclip)))
    (:SurfaceType4
      (LocalVariables|Setclip (Variables|Default|GetMetalSound))
      (return (LocalVariables|Getclip)))
    (:SurfaceType5
      (LocalVariables|Setclip (Variables|Default|GetGlassSound)))))