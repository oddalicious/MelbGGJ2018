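; WinPoint is the level goal actor in the cup game, marked by a cube that bobs on a sine wave and spins every tick.
; Its box overlap stores a CupCharacter that enters with a positive FillAmount and clears it on exit.
; While overlapped, Tick waits until the cup is not noticeable, then shows its win widget once.
; A separate WinTheGame function quits the game but is not called within this graph.
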(event OnComponentBeginOverlap(Box)
  (params (OverlappedComponent :type Primitive%20Component%20Object%20Reference) (OtherActor :type Actor%20Object%20Reference) (OtherComp :type Primitive%20Component%20Object%20Reference) (OtherBodyIndex :type Integer) (bFromSweep :type Boolean) (SweepResult :type Hit%20Result%20Structure%20%28by%20ref%29))
  (bind _ascup_character (Utilities|Casting|CastToCupCharacter OtherActor))
  (if (> (Variables|/Game/CupGame/Blueprints/CupCharacter.CupCharacter_C|GetfillAmount _ascup_character) 0.0)
    (Variables|Default|Setoverlapped true)
    (Variables|Default|Setcup _ascup_character)))

(event OnComponentEndOverlap(Box)
  (params (OverlappedComponent :type Primitive%20Component%20Object%20Reference) (OtherActor :type Actor%20Object%20Reference) (OtherComp :type Primitive%20Component%20Object%20Reference) (OtherBodyIndex :type Integer))
  (Utilities|Casting|CastToCupCharacter OtherActor)
  (Variables|Default|Setoverlapped false)
  (Variables|Default|Setcup 0))

(event EventBeginPlay
  (Variables|Default|SetcubeHeight (.z (Variables|/Script/Engine.SceneComponent|GetRelativeLocation (Variables|Default|GetCube)))))

(event EventTick
  (params (DeltaSeconds :type Float%20%28single-precision%29))
  (bind _cup (Variables|Default|Getcup))
  (CallFunction|SetBoxPosition DeltaSeconds)
  (if (Variables|Default|Getoverlapped)
    (bind _ouytput (Default|IsNoticeAbleFunc _cup))
    (if (not _ouytput)
      (Utilities|FlowControl|DoOnce false
        (:Completed
          (Default|ShowWinWidget _cup))))))

(fn ConstructionScript)

(fn WintheGame
  (Game|QuitGame 0 "Quit"))

(fn SetBoxPosition
  (params (A :type Float%20%28single-precision%29))
  (bind _cube (Variables|Default|GetCube))
  (bind _relativerotation (Variables|/Script/Engine.SceneComponent|GetRelativeRotation _cube))
  (bind _output_get (Variables|Default|SetcurrentTime (+ (* A (Variables|Default|Getspeed)) (Variables|Default|GetcurrentTime))))
  (Transformation|SetRelativeLocation (Variables|Default|GetCube) (Math|Vector|MakeVector 0.0 0.0 (+ (Variables|Default|GetcubeHeight) (* (Math|Trig|Sin(Radians) _output_get) (Variables|Default|Getheight)))) false false)
  (Transformation|SetRelativeRotation _cube (Math|Rotator|MakeRotator (.roll _relativerotation) (.pitch _relativerotation) (+ (.yaw _relativerotation) (* (Variables|Default|GetrotateSpeed) A))) false false))