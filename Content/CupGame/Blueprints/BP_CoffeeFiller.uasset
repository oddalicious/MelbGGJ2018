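; Coffee machine actor for the cup game that fills a CupCharacter standing in its trigger box, then activates the WinPoint.
; Once the cup is ready, it locks cup movement and plays a prepare stage, progressively recoloring its lights, followed by a fill stage.
; Sound durations time both stages; during filling, Tick feeds the cup and widens the stream cylinder along a sine curve, then hides it and frees the cup.
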(event OnComponentBeginOverlap(Box)
  (params (OverlappedComponent :type Primitive%20Component%20Object%20Reference) (OtherActor :type Actor%20Object%20Reference) (OtherComp :type Primitive%20Component%20Object%20Reference) (OtherBodyIndex :type Integer) (bFromSweep :type Boolean) (SweepResult :type Hit%20Result%20Structure%20%28by%20ref%29))
  (bind _ascup_character (Utilities|Casting|CastToCupCharacter OtherActor))
  (Variables|Default|SetCup _ascup_character)
  (Variables|Default|SetcanFill true))

(event OnComponentEndOverlap(Box)
  (params (OverlappedComponent :type Primitive%20Component%20Object%20Reference) (OtherActor :type Actor%20Object%20Reference) (OtherComp :type Primitive%20Component%20Object%20Reference) (OtherBodyIndex :type Integer))
  (Utilities|Casting|CastToCupCharacter OtherActor)
  (Variables|Default|SetcanFill false)
  (Variables|Default|SetCup 0))

(event Custom|BeginFill
  (CallFunction|PerformStageOne)
  (Utilities|FlowControl|Delay (Variables|/Script/Engine.SoundBase|GetDuration (Variables|Default|GetPrepareSound)))
  (CallFunction|PerformStage2)
  (Utilities|FlowControl|Delay (Variables|/Script/Engine.SoundBase|GetDuration (Variables|Default|GetFill%20Sound)))
  (Variables|Default|SetisFilling false)
  (Variables|/Game/CupGame/Blueprints/CupCharacter.CupCharacter_C|SetcanMove (Variables|Default|GetCup) true)
  (Rendering|SetVisibility (Variables|Default|GetCylinder) false false)
  (Components|Activation|SetActive (Variables|/Game/CupGame/Blueprints/WinPoint.WinPoint_C|GetDefaultSceneRoot (Variables|Default|GetwinPoint)) true false))

(event EventBeginPlay
  (Components|Activation|SetActive (Variables|Default|GetDefaultSceneRoot) false false))

(event EventTick
  (params (DeltaSeconds :type Float%20%28single-precision%29))
  (if (Variables|Default|GetcanFill)
    (if (.Output (Utilities|CupReady))
      (if (Variables|Default|GetisFilling)
        (if (Variables|Default|GetisFilling)
          (Default|Fill (Variables|Default|GetCup) DeltaSeconds (Variables|/Script/Engine.SoundBase|GetDuration (Variables|Default|GetFill%20Sound)))
          (CallFunction|PerformFill DeltaSeconds))
        (else
          (Utilities|FlowControl|Sequence
            (:then_0
              (Utilities|FlowControl|DoOnce false
                (:Completed
                  (CallFunction|BeginFill))))
            (:then_1
              (CallFunction|FillLights DeltaSeconds))))))))

(fn ConstructionScript)

(fn PerformStageOne
  (Variables|Default|Setpreparing true)
  (Variables|/Game/CupGame/Blueprints/CupCharacter.CupCharacter_C|SetcanMove (Variables|Default|GetCup) false)
  (Audio|PlaySoundatLocation self (Variables|Default|GetPrepareSound) (Transformation|GetWorldLocation (Variables|Default|GetCylinder))))

(fn PerformStage2
  (Variables|Default|Setpreparing false)
  (Audio|PlaySound2D self (Variables|Default|GetFill%20Sound))
  (Variables|Default|SetisFilling true))

(fn PerformFill
  (params (DeltaTime :type Float%20%28single-precision%29))
  (bind _output_get (Variables|Default|SetfillTime (+ (Variables|Default|GetfillTime) DeltaTime)))
  (Transformation|SetWorldScale3D (Variables|Default|GetCylinder) (Math|Vector|MakeVector (.x (* (Variables|Default|GetcylindermaxTransform) (Math|Trig|Sin(Radians) (Math|Float|Clamp(Float) (/ _output_get (Variables|/Script/Engine.SoundBase|GetDuration (Variables|Default|GetFill%20Sound))))))) (.y (* (Variables|Default|GetcylindermaxTransform) (Math|Trig|Sin(Radians) (Math|Float|Clamp(Float) (/ _output_get (Variables|/Script/Engine.SoundBase|GetDuration (Variables|Default|GetFill%20Sound))))))) (.z (Transformation|GetWorldScale (Variables|Default|GetCylinder))))))

(fn FillLights
  (params (deltaTime :type Float%20%28single-precision%29))
  (bind _lights (Variables|Default|Getlights))
  (bind _returnvalue (Utilities|Array|Length _lights))
  (bind _returnvalue_2 (- _returnvalue 1))
  (if (Variables|Default|Getpreparing)
    (bind _output_get (Variables|Default|SetlightTime (+ (Variables|Default|GetlightTime) deltaTime)))
    (if (> _returnvalue 0)
      (Rendering|Components|Light|SetLightColor (Variables|/Script/Engine.Light|GetLightComponent (Utilities|Array|Get(acopy) _lights (Math|Integer|Clamp(Integer) (Math|Float|Truncate (* _returnvalue_2 (Math|Float|Clamp(Float) (/ _output_get (Variables|/Script/Engine.SoundBase|GetDuration (Variables|Default|GetPrepareSound)))))) 0 _returnvalue_2))) (Variables|Default|GetDoneColor) true))))