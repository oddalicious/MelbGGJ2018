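; Watcher actor for the cup game that spots the player in its linked trigger zones and shows the lose widget after prolonged detection.
; A spot timer rises while several line traces across the capsule's width hit a moving, rotating or animating player, and decays otherwise.
; The timer drives spotlight color and aim, while notice and give-up transitions fire sounds, animation messages and MusicManager calls.
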(event Custom|BeginSpot)

(event EventBeginPlay
  (CallFunction|SubscribeTriggers)
  (bind _ascup_game_mode (Utilities|Casting|CastToCupGameMode (Game|GetGameMode)))
  (Variables|Default|SetgameMode _ascup_game_mode))

(event EventTick
  (params (DeltaSeconds :type Float%20%28single-precision%29))
  (CallFunction|ScaleEyestoTarget)
  (bind _percentspotted (CallFunction|CheckTime DeltaSeconds))
  (CallFunction|CheckPlayerLoss)
  (Rendering|Components|Light|SetLightColor (Variables|Default|GetSpotLight) (Math|Color|Lerp(LinearColor) (Variables|Default|GetsafeColor) (Variables|Default|GetdangerColor) _percentspotted) true)
  (if (Utilities|AnyTriggersActive)
    (Variables|Default|SettimeSinceSpot (+ (Variables|Default|GettimeSinceSpot) DeltaSeconds))))

(fn ConstructionScript)

(fn CheckTime
  (params (Delta%20Time :type Float%20%28single-precision%29))
  (bind _timetonoticeplayer (Variables|Default|GettimeToNoticePlayer))
  (LocalVariables|SetdeltaTime Delta%20Time)
  (Utilities|IsValid (Variables|Default|GetgameMode)
    (:Is%20Valid
      (LocalVariables|SetcurrentSpotPercent (/ (Variables|Default|GetcurrentSpotTime) (Variables|/Game/CupGame/Blueprints/CupGameMode.CupGameMode_C|GetSpotTime (Variables|Default|GetgameMode))))
      (Utilities|SpottingMacro
        (:Trigger%20Active%20and%20Noticeable
          (if (and (< (Variables|Default|GetcurrentSpotTime) _timetonoticeplayer) (>= (+ (Variables|Default|GetcurrentSpotTime) (LocalVariables|GetdeltaTime)) _timetonoticeplayer))
            (CallFunction|SpotPlayer))
          (bind _output_get (Variables|Default|SetcurrentSpotTime (+ (Variables|Default|GetcurrentSpotTime) (LocalVariables|GetdeltaTime))))
          (Variables|Default|SetcanBeAnnoyed (> _output_get 2.0)))
        (:Trigger%20Active%20and%20not%20Noticeable
          (if (and (> (Variables|Default|GetcurrentSpotTime) 0.0) (<= (Math|Float|Max(Float) (- (Variables|Default|GetcurrentSpotTime) (/ (LocalVariables|GetdeltaTime) (Variables|Default|GetReduceSpeed))) 0.0) 0.0)) :!label _label
            (CallFunction|GiveUp))
          (Variables|Default|SetcurrentSpotTime (Math|Float|Max(Float) (- (Variables|Default|GetcurrentSpotTime) (/ (LocalVariables|GetdeltaTime) (Variables|Default|GetReduceSpeed))) 0.0)))
        (:No%20Triggers%20Active
          (goto _label)))
      (return (Math|Float|Clamp(Float) (LocalVariables|GetcurrentSpotPercent))))))

(fn GiveUp
  (bind _giveupsound (Variables|Default|GetGiveUpSound))
  (if (Variables|Default|GetcanBeAnnoyed)
    (Audio|PlaySoundatLocation self (Utilities|Array|Get(acopy) _giveupsound (Math|Random|RandomInteger (Utilities|Array|Length _giveupsound))) (Transformation|GetActorLocation)))
  (Class|AnimInterface|AIEndSpot(Message) (Components|SkeletalMesh|GetAnimInstance (Variables|Default|GetSkeletalMesh)))
  (bind _outactors (Actor|GetAllActorsOfClass "/Game/CupGame/Blueprints/MusicManager.MusicManager_C"))
  (Default|LoseSpot (Utilities|Array|Get(acopy) _outactors)))

(fn SpotPlayer
  (bind _outactors (Actor|GetAllActorsOfClass "/Game/CupGame/Blueprints/MusicManager.MusicManager_C"))
  (Default|HasBeenSpotted (Utilities|Array|Get(acopy) _outactors))
  (Audio|PlaySoundatLocation self (Utilities|Array|Get(acopy) (Variables|Default|GetHuhSounds)) (Transformation|GetActorLocation))
  (Class|AnimInterface|AIBeginSpot(Message) (Components|SkeletalMesh|GetAnimInstance (Variables|Default|GetSkeletalMesh)))
  (Variables|Default|SettimeSinceSpot 0.0))

(fn SubscribeTriggers
  (for _array_element (Variables|Default|GetTriggerZones)
    (Utilities|IsValid _array_element
      (:Is%20Valid
        (Collision|BindEventtoOnActorBeginOverlap _array_element (EventDispatchers|CreateEvent :!event ActorBeginOverlap))
        (Collision|BindEventtoOnActorEndOverlap _array_element (EventDispatchers|CreateEvent :!event ActorEndOverlap))))))

(fn ActorBeginOverlap
  (params (Trigger :type Actor%20Object%20Reference) (Overlapped :type Actor%20Object%20Reference))
  (bind _ascup_character (Utilities|Casting|CastToCupCharacter Overlapped))
  (Math|Integer|IncrementInt (Variables|Default|GetActiveTriggers)
    (:%20%20
      (Variables|Default|SetCupCharacter _ascup_character))))

(fn ActorEndOverlap
  (params (Trigger :type Actor%20Object%20Reference) (Overlapped :type Actor%20Object%20Reference))
  (Utilities|Casting|CastToCupCharacter Overlapped)
  (bind _result (Math|Integer|DecrementInt (Variables|Default|GetActiveTriggers))
    (:%20%20
      (bind _output_get (Variables|Default|SetActiveTriggers (Math|Integer|Max(Integer) _result)))
      (if (== _output_get 0)
        (Variables|Default|SetCupCharacter 0)
        (Development|PrintString (LocalVariables|GetTrigger%20Disconnected))
        (Development|PrintString (Utilities|String|ToString(Integer) _output_get))))))

(fn CheckPlayerLoss
  (bind _cupcharacter (Variables|Default|GetCupCharacter))
  (if (>= (Variables|Default|GetcurrentSpotTime) (Variables|Default|GetLossTime))
    (Utilities|IsValid _cupcharacter
      (:Is%20Valid
        (Default|ShowLoseWidget _cupcharacter)))))

(fn ScaleEyestoTarget
  (bind _spotlight (Variables|Default|GetSpotLight))
  (if (and (Utilities|AnyTriggersActive) (> (Variables|Default|GetcurrentSpotTime) 1.0))
    (LocalVariables|SetTargetLocation (Transformation|GetActorLocation (Variables|Default|GetCupCharacter)))
    (else
      (LocalVariables|SetTargetLocation (Transformation|GetWorldLocation (Variables|Default|GetRegularTarget)))))
  (Transformation|SetWorldRotation _spotlight (Math|Rotator|MakeRotator (.roll (Math|Rotator|FindLookatRotation (Transformation|GetWorldLocation _spotlight) (LocalVariables|GetTargetLocation))) (.pitch (Math|Rotator|FindLookatRotation (Transformation|GetWorldLocation _spotlight) (LocalVariables|GetTargetLocation))) (.yaw (Math|Rotator|FindLookatRotation (Transformation|GetWorldLocation _spotlight) (LocalVariables|GetTargetLocation)))) false false))

(fn IsPlayerVisible
  (bind _cupcharacter (Variables|Default|GetCupCharacter))
  (bind _returnvalue (Transformation|GetActorLocation _cupcharacter))
  (if (Utilities|AnyTriggersActive)
    (LocalVariables|SethitRays 0)
    (bind _output_get (LocalVariables|SetRightVector (* (Math|Vector|GetRightVector (Math|Rotator|FindLookatRotation (Transformation|GetWorldLocation (Variables|Default|GetSpotLight)) _returnvalue)) (.OutRadius (Class|CapsuleComponent|GetUnscaledCapsuleSizeWithoutHemisphere (Variables|/Script/Engine.Character|GetCapsuleComponent _cupcharacter))))))
    (for _array_element (Variables|Default|Getrays)
      (bind (_outhit _returnvalue_2) (Collision|LineTraceByChannel (Transformation|GetWorldLocation (Variables|Default|GetSpotLight)) (+ _returnvalue (* _output_get _array_element)) "TraceTypeQuery1" true 0 (select (> (Variables|Default|GetcurrentSpotTime) 0.0) "ForOneFrame" "None")))
      (if _returnvalue_2
        (if (== (.hitactor _outhit) (Variables|Default|GetCupCharacter))
          (Math|Integer|IncrementInt (LocalVariables|GethitRays)))))
    (return (> (LocalVariables|GethitRays) 1))))